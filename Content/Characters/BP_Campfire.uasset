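; BP_Campfire is a rest-site pickup that heals the player and opens the map when touched.
; When an STSCharacter overlaps its sphere, it restores 30% of max health, clamped, on the STSGameMode, which stores the health values.
; It then refreshes the main UI's HP display, adds a new WBP_Map widget to the viewport and destroys itself.
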(event OnComponentBeginOverlap(Sphere1)
  (params (OverlappedComponent :type Primitive%20Component%20Object%20Reference) (OtherActor :type Actor%20Object%20Reference) (OtherComp :type Primitive%20Component%20Object%20Reference) (OtherBodyIndex :type Integer) (bFromSweep :type Boolean) (SweepResult :type Hit%20Result%20Structure%20%28by%20ref%29))
  (Utilities|Casting|CastToSTSCharacter OtherActor)
  (bind _asstsgame_mode (Utilities|Casting|CastToSTSGameMode (Game|GetGameMode)))
  (bind _output_get (Variables|/Script/STS.STSGameMode|SetCurrentHealth _asstsgame_mode (Math|Integer|Clamp(Integer) (+ (Variables|/Script/STS.STSGameMode|GetCurrentHealth _asstsgame_mode) (* (Math|Conversions|ToFloat(Integer) (Variables|/Script/STS.STSGameMode|GetMaxHealth _asstsgame_mode)) 0.3)) 0 (Variables|/Script/STS.STSGameMode|GetMaxHealth _asstsgame_mode))))
  (Class|STSUserWidget|UpdatePlayerHP (Variables|/Script/STS.STSGameMode|GetMainUIWidget _asstsgame_mode) _output_get (Variables|/Script/STS.STSGameMode|GetMaxHealth _asstsgame_mode))
  (bind _returnvalue (UserInterface|CreateWidget "/Game/Characters/WBP_Map.WBP_Map_C"))
  (UserInterface|Viewport|AddtoViewport _returnvalue 0)
  (Actor|DestroyActor))

(event EventBeginPlay)

(event Collision|EventActorBeginOverlap
  (params (OtherActor :type Actor%20Object%20Reference)))

(event EventTick
  (params (DeltaSeconds :type Float%20%28single-precision%29)))

(fn ConstructionScript)