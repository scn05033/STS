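; BP_Anvil is a card-upgrade station that opens the smith selection panel when the player character overlaps its sphere.
; The overlap destroys campfires and, inside that same loop, shows the panel, switches to UI-only input and blocks movement and look, so nothing opens without a campfire.
; It rebuilds the card list from the GameMode's master deck, adding smithing-mode widgets only for cards with an upgrade in CardData, then destroys itself.
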(event OnComponentBeginOverlap(Sphere1)
  (params (OverlappedComponent :type Primitive%20Component%20Object%20Reference) (OtherActor :type Actor%20Object%20Reference) (OtherComp :type Primitive%20Component%20Object%20Reference) (OtherBodyIndex :type Integer) (bFromSweep :type Boolean) (SweepResult :type Hit%20Result%20Structure%20%28by%20ref%29))
  (bind _returnvalue (Game|GetPlayerController 0))
  (Utilities|Casting|CastToSTSCharacter OtherActor
    (:then
      (bind _outactors (Actor|GetAllActorsOfClass "/Game/Characters/BP_Campfire.BP_Campfire_C"))
      (for _array_element _outactors
        (Actor|DestroyActor _array_element)
        (bind _asstsgame_mode (Utilities|Casting|CastToSTSGameMode (Game|GetGameMode)))
        (bind _asstswidget (Utilities|Casting|CastToSTSWidget (Variables|/Script/STS.STSGameMode|GetMainUIWidget _asstsgame_mode))
          (:then
            (Widget|SetVisibility (Variables|/Game/Characters/STSWidget.STSWidget_C|GetSmithSelectPanel _asstswidget) "Visible")
            (Variables|/Script/Engine.PlayerController|SetbShowMouseCursor _returnvalue true)
            (Input|SetInputModeUIOnly _returnvalue 0 "DoNotLock" false)
            (Input|SetIgnoreMoveInput _returnvalue true)
            (Input|SetIgnoreLookInput _returnvalue true)
            (Widget|Panel|ClearChildren (Variables|/Game/Characters/STSWidget.STSWidget_C|GetBox_DeckList _asstswidget))
            (for (_array_element_2 _array_index) (Variables|/Script/STS.STSGameMode|GetMasterDeck _asstsgame_mode)
              (bind _returnvalue_2 (Utilities|GetDataTableRow "/Game/Characters/CardData.CardData" _array_element_2)
                (:then
                  (if (!= (.UpgradedCardID (Utilities|Struct|BreakCardData _returnvalue_2)) "")
                    (Development|PrintString "카드 생성 중")
                    (bind _returnvalue_3 (UserInterface|CreateWidget "/Game/Characters/WBP_TestCard.WBP_TestCard_C" 0 _array_element_2 _array_index))
                    (Variables|/Script/STS.STSCardWidget|SetbIsSmithingMode _returnvalue_3 true)
                    (Widget|Panel|AddChild (Variables|/Game/Characters/STSWidget.STSWidget_C|GetBox_DeckList _asstswidget) _returnvalue_3)))))
            (Actor|DestroyActor))
          (:CastFailed
            (Development|PrintString "UI 변수가 비어있음")))))
    (:CastFailed
      (Development|PrintString "캐릭터 캐스팅 실패"))))

(event EventBeginPlay)

(event Collision|EventActorBeginOverlap
  (params (OtherActor :type Actor%20Object%20Reference)))

(event EventTick
  (params (DeltaSeconds :type Float%20%28single-precision%29)))

(fn ConstructionScript)